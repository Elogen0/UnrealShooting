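; Base Blueprint for a multiplayer shooter character, handling movement input, armed aim-offset and turn-in-place state, and combat montages.
; The locally controlled character computes aim yaw and interpolated turning each tick while a weapon is equipped.
; Other instances infer turns from actor yaw deltas on a throttled timer and remap compressed replicated pitch.
; Montage events cover fire, hit react, per-weapon reload, and elimination with a timeline-driven dissolve on dynamic materials.
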(event `self.ReceiveBeginPlay`
  (`parent.ReceiveBeginPlay`)
  (`|ExecutionSequence`
    (:`then_0`
      (if (`self.IsLocallyControlled`)
        (bind _asb_alpha_player_controller (cast `/Game/Blueprints/Characters/B_AlphaPlayerController` (`self.GetController`)))
        (`EnhancedInputSubsystemInterface.AddMappingContext` (pcsubsystem `EnhancedInputLocalPlayerSubsystem` _asb_alpha_player_controller) "/Game/Input/IMC_Player.IMC_Player" 0 (struct))))))

(event `self.ReceiveTick`
  (params (DeltaSeconds :type "Float (single-precision)"))
  (`parent.ReceiveTick` DeltaSeconds)
  (if (and (> (`self.GetLocalRole`) 1) (`self.IsLocallyControlled`))
    (`self.AimOffset` DeltaSeconds)
    (else
      (`|ExecutionSequence`
        (:`then_0`
          (bind _output_get (set `self.TimeSinceLastMovemntReplication` (+ DeltaSeconds (`self.TimeSinceLastMovemntReplication`))))
          (if (> _output_get 0.25)
            (`self.BP_ReplicatedMovement`)))
        (:`then_1`
          (`self.CalculateAimOffsetPitch`))))))

(event `EnhancedInput|/Game/Input/IA_Move`
  (params (ActionValue :type "Vector2D Structure") (ElapsedSeconds :type "Float (double-precision)") (TriggeredSeconds :type "Float (double-precision)") (InputAction :type "InputAction Object Reference" :default "/Game/Input/IA_Move.IA_Move"))
  (bind (_x _y) (`KismetMathLibrary.BreakVector2D` ActionValue))
  (bind _returnvalue (`Controller.GetControlRotation` (`self.GetController`)))
  (:`Triggered`
    (`|ExecutionSequence`
      (:`then_0`
        (`self.AddMovementInput` (`KismetMathLibrary.GetRightVector` _returnvalue) _x))
      (:`then_1`
        (`self.AddMovementInput` (`KismetMathLibrary.GetForwardVector` _returnvalue) _y)))))

(event `self.BP_ReplicatedMovement`
  (`self.SimProxyTurn`)
  (set `self.TimeSinceLastMovemntReplication` 0.0))

(event `self.PlayFireMontage`
  (params (bAiming :type Boolean))
  (bind _returnvalue (`SkeletalMeshComponent.GetAnimInstance` (`self.Mesh`)))
  (`AnimInstance.Montage_Play` _returnvalue "/Game/Blueprints/Characters/Animation/AM_FireWeapon.AM_FireWeapon" 1.0 "MontageLength" 0.0 true)
  (if bAiming
    (`AnimInstance.Montage_JumpToSection` _returnvalue "RifleAim" null)
    (else
      (`AnimInstance.Montage_JumpToSection` _returnvalue "RifleHip" null))))

(event `self.PlayHitReactMontage`
  (`AnimInstance.Montage_Play` (`SkeletalMeshComponent.GetAnimInstance` (`self.Mesh`)) "/Game/Blueprints/Characters/Animation/AM_HitReact.AM_HitReact" 1.0 "MontageLength" 0.0 true))

(event `self.PlayReloadMontage`
  (params (WeaponTYpe :type "EWeaponType Enum" :default "EWT_AssaultRifle"))
  (bind _returnvalue (`SkeletalMeshComponent.GetAnimInstance` (`self.Mesh`)))
  (`AnimInstance.Montage_Play` _returnvalue "/Game/Blueprints/Characters/Animation/AM_Reload.AM_Reload" 1.0 "MontageLength" 0.0 true)
  (switch `EWeaponType` WeaponTYpe
    (:`EWT_AssaultRifle`
      (`AnimInstance.Montage_JumpToSection` _returnvalue "Rifle" "/Game/Blueprints/Characters/Animation/AM_Reload.AM_Reload" :!label _label))
    (:`EWT_RocketLauncher`
      (goto _label))
    (:`EWT_Pistol`
      (`AnimInstance.Montage_JumpToSection` _returnvalue "Pistol" "/Game/Blueprints/Characters/Animation/AM_Reload.AM_Reload" :!label _label_2))
    (:`EWT_SubmachineGun`
      (goto _label_2))
    (:`EWT_Shotgun`
      (`AnimInstance.Montage_JumpToSection` _returnvalue "Shotgun" "/Game/Blueprints/Characters/Animation/AM_Reload.AM_Reload"))
    (:`EWT_SniperRifle`
      (goto _label))
    (:`EWT_GranadeLauncher`
      (goto _label))))

(event `self.PlayElimMontage`
  (`|ExecutionSequence`
    (:`then_0`
      (`AnimInstance.Montage_Play` (`SkeletalMeshComponent.GetAnimInstance` (`self.Mesh`)) "/Game/Blueprints/Characters/Animation/AM_Elim.AM_Elim" 1.0 "MontageLength" 0.0 true))
    (:`then_1`
      (bind _returnvalue (`KismetMaterialLibrary.CreateDynamicMaterialInstance` "/Game/Assets/Mixamo/Material/M_AlphaCharacterDissolve.M_AlphaCharacterDissolve"))
      (`PrimitiveComponent.SetMaterial` (`self.Mesh`) 0 _returnvalue)
      (`MaterialInstanceDynamic.SetScalarParameterValue` _returnvalue "Dissolve" 0.55)
      (`MaterialInstanceDynamic.SetScalarParameterValue` _returnvalue "Glow" 200.0))
    (:`then_2`
      (bind _returnvalue_2 (`KismetMaterialLibrary.CreateDynamicMaterialInstance` "/Game/Assets/Mixamo/Material/M_AlphaCharacterDissolve2.M_AlphaCharacterDissolve2"))
      (`PrimitiveComponent.SetMaterial` (`self.Mesh`) 1 _returnvalue_2)
      (`MaterialInstanceDynamic.SetScalarParameterValue` _returnvalue_2 "Dissolve" 0.55)
      (`MaterialInstanceDynamic.SetScalarParameterValue` _returnvalue_2 "Glow" 200.0))
    (:`then_3`
      (bind (_direction _dissolvecurve) (`Timeline|Timeline` :`NewTime` (`GameplayStatics.GetWorldDeltaSeconds`))
        (:`Update`
          (`MaterialInstanceDynamic.SetScalarParameterValue` _returnvalue "Dissolve" _dissolvecurve)
          (`MaterialInstanceDynamic.SetScalarParameterValue` _returnvalue_2 "Dissolve" _dissolvecurve))))))

(fn `AimOffset`
  (params (DeltaTime :type "Float (double-precision)"))
  (locals (Velocity :type "Vector Structure") (Speed :type "Float (double-precision)"))
  (bind (_returnvalue_roll _returnvalue_pitch _returnvalue_yaw) (`KismetMathLibrary.BreakRotator` (`self.GetBaseAimRotation`)))
  (bind (_returnvalue_roll_2 _returnvalue_pitch_2 _returnvalue_yaw_2) (`KismetMathLibrary.BreakRotator` (`self.GetBaseAimRotation`)))
  (bind _charactermovement (`self.CharacterMovement`))
  (bind _combat (`self.Combat`))
  (bind (_returnvalue_roll_3 _returnvalue_pitch_3 _returnvalue_yaw_3) (`KismetMathLibrary.BreakRotator` (`KismetMathLibrary.NormalizedDeltaRotator` (`KismetMathLibrary.MakeRotator` 0.0 0.0 _returnvalue_yaw_2) (`self.StartingAimRotation`))))
  (`/Engine/EditorBlueprintResources/StandardMacros.IsValid` _combat
    (:`Is Valid`
      (`/Engine/EditorBlueprintResources/StandardMacros.IsValid` (`CombatComponent.EquippedWeapon` _combat)
        (:`Is Valid`
          (set `local.Speed` (`self.CalculateMovementSpeed`))
          (`|ExecutionSequence`
            (:`then_0`
              ;[1 1 1] Statind still, not Jumping
              (if (and (== (`local.Speed`) 0.0) (not (`NavMovementComponent.IsFalling` _charactermovement)))
                (set `self.bRotateRootBone` true)
                (set `self.AO_Yaw` _returnvalue_yaw_3)
                (`|ExecutionSequence`
                  (:`then_0`
                    (if (`|EnumEquality` (`self.TurningInPlace`) "ETIP_NotTurning")
                      (set `self.InterpAOYaw` (`self.AO_Yaw`))))
                  (:`then_1`
                    (set `self.bUseControllerRotationYaw` true)
                    (`self.TurnInPlace` (`local.DeltaTime`))))))
            (:`then_1`
              ;[1 1 1] Running, or Jumping
              (if (or (> (`local.Speed`) 0.0) (`NavMovementComponent.IsFalling` _charactermovement))
                (set `self.bRotateRootBone` false)
                (set `self.StartingAimRotation` (`KismetMathLibrary.MakeRotator` 0.0 0.0 _returnvalue_yaw))
                (set `self.AO_Yaw` 0.0)
                (set `self.bUseControllerRotationYaw` true)
                (set `self.TurningInPlace` "ETIP_NotTurning")))
            (:`then_2`
              (`self.CalculateAimOffsetPitch`))))))))

(fn `CalculateAimOffsetPitch`
  (bind (_returnvalue_roll _returnvalue_pitch) (`KismetMathLibrary.BreakRotator` (`self.GetBaseAimRotation`)))
  (set `self.AO_Pitch` _returnvalue_pitch)
  ;[1 1 1] ReCalculating Compressed Rotator to Correct Rotator
  (if (and (> (`self.AO_Pitch`) 90.0) (not (`self.IsLocallyControlled`)))
    (set `self.AO_Pitch` (`KismetMathLibrary.MapRangeClamped` (`self.AO_Pitch`) 270.0 360.0 -90.0))))

(fn `SimProxyTurn`
  (bind _combat (`self.Combat`))
  (`/Engine/EditorBlueprintResources/StandardMacros.IsValid` _combat
    (:`Is Valid`
      (`/Engine/EditorBlueprintResources/StandardMacros.IsValid` (`CombatComponent.EquippedWeapon` _combat)
        (:`Is Valid`
          (set `self.bRotateRootBone` false)
          (if (> (`self.CalculateMovementSpeed`) 0.0)
            (set `self.TurningInPlace` "ETIP_NotTurning")
            (else
              (`self.CalculateAimOffsetPitch`)
              (bind _output_get (set `self.PorxyRotationLastFrame` (`self.ProxyRotation`)))
              (bind _output_get_2 (set `self.ProxyRotation` (`self.K2_GetActorRotation`)))
              (bind (_returnvalue_roll _returnvalue_pitch _returnvalue_yaw) (`KismetMathLibrary.BreakRotator` (`KismetMathLibrary.NormalizedDeltaRotator` _output_get_2 _output_get)))
              (set `self.ProxyYaw` _returnvalue_yaw)
              (if (> (`self.ProxyYaw`) (`self.TurnThreshold`))
                (set `self.TurningInPlace` "ETIP_Right")
                (elif (< (`self.ProxyYaw`) (* -1.0 (`self.TurnThreshold`)))
                  (set `self.TurningInPlace` "ETIP_Left")
                  (else
                    (set `self.TurningInPlace` "ETIP_NotTurning")))))))))))

(fn `TurnInPlace`
  (params (DeltaTime :type "Float (double-precision)"))
  (bind (_returnvalue_roll _returnvalue_pitch _returnvalue_yaw) (`KismetMathLibrary.BreakRotator` (`self.GetBaseAimRotation`)))
  (`|ExecutionSequence`
    (:`then_0`
      (if (> (`self.AO_Yaw`) 90.0)
        (set `self.TurningInPlace` "ETIP_Right")
        (elif (< (`self.AO_Yaw`) -90.0)
          (set `self.TurningInPlace` "ETIP_Left"))))
    (:`then_1`
      (if (`|EnumInequality` (`self.TurningInPlace`) "ETIP_NotTurning")
        (bind _output_get (set `self.InterpAOYaw` (`KismetMathLibrary.FInterpTo` (`self.InterpAOYaw`) 0.0 (`local.DeltaTime`) 4.0)))
        (bind _output_get_2 (set `self.AO_Yaw` _output_get))
        (if (< (`KismetMathLibrary.Abs` _output_get_2) 15.0)
          (set `self.TurningInPlace` "ETIP_NotTurning")
          (set `self.StartingAimRotation` (`KismetMathLibrary.MakeRotator` 0.0 0.0 _returnvalue_yaw)))))))

(fn `UserConstructionScript`)