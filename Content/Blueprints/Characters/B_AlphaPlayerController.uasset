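; Player controller that turns Enhanced Input actions into commands for the controlled B_AlphaCharacterBase pawn.
; Look feeds yaw and pitch directly; other actions cast the pawn, then trigger jump, crouch toggle or equip.
; Aim and fire forward press and release states to the character's Combat component, with fire cancel and completion both releasing the trigger.
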(event `self.ReceiveBeginPlay`)

(event `self.ReceivePossess`
  (params (PossessedPawn :type "Pawn Object Reference")))

(event `EnhancedInput|/Game/Input/IA_Look`
  (params (ActionValue :type "Vector2D Structure") (ElapsedSeconds :type "Float (double-precision)") (TriggeredSeconds :type "Float (double-precision)") (InputAction :type "InputAction Object Reference" :default "/Game/Input/IA_Look.IA_Look"))
  (bind (_x _y) (`KismetMathLibrary.BreakVector2D` ActionValue))
  (:`Triggered`
    (`|ExecutionSequence`
      (:`then_0`
        (`self.AddYawInput` _x))
      (:`then_1`
        (`self.AddPitchInput` _y)))))

(event `EnhancedInput|/Game/Input/IA_Jump`
  (params (ActionValue :type Boolean) (ElapsedSeconds :type "Float (double-precision)") (TriggeredSeconds :type "Float (double-precision)") (InputAction :type "InputAction Object Reference" :default "/Game/Input/IA_Jump.IA_Jump"))
  (:`Triggered`
    (bind _asb_alpha_character_base (cast `/Game/Blueprints/Characters/B_AlphaCharacterBase` (`self.K2_GetPawn`)))
    (if (`Character.CanJump` _asb_alpha_character_base)
      (`Character.Jump` _asb_alpha_character_base))))

(event `EnhancedInput|/Game/Input/IA_Equipp`
  (params (ActionValue :type Boolean) (ElapsedSeconds :type "Float (double-precision)") (TriggeredSeconds :type "Float (double-precision)") (InputAction :type "InputAction Object Reference" :default "/Game/Input/IA_Equipp.IA_Equipp"))
  (:`Started`
    (bind _asb_alpha_character_base (cast `/Game/Blueprints/Characters/B_AlphaCharacterBase` (`self.K2_GetPawn`)))
    (`AlphaCharacter.EquipButtonPressed` _asb_alpha_character_base)))

(event `EnhancedInput|/Game/Input/IA_Crouch`
  (params (ActionValue :type Boolean) (ElapsedSeconds :type "Float (double-precision)") (TriggeredSeconds :type "Float (double-precision)") (InputAction :type "InputAction Object Reference" :default "/Game/Input/IA_Crouch.IA_Crouch"))
  (:`Started`
    (bind _asb_alpha_character_base (cast `/Game/Blueprints/Characters/B_AlphaCharacterBase` (`self.K2_GetPawn`)))
    (if (`Character.bIsCrouched` _asb_alpha_character_base)
      (`Character.UnCrouch` _asb_alpha_character_base)
      (`Character.UnCrouch` _asb_alpha_character_base)
      (elif (`Character.CanCrouch` _asb_alpha_character_base)
        (`Character.Crouch` _asb_alpha_character_base)))))

(event `EnhancedInput|/Game/Input/IA_Aim`
  (params (ActionValue :type Boolean) (ElapsedSeconds :type "Float (double-precision)") (TriggeredSeconds :type "Float (double-precision)") (InputAction :type "InputAction Object Reference" :default "/Game/Input/IA_Aim.IA_Aim"))
  (:`Started`
    (bind _asb_alpha_character_base (cast `/Game/Blueprints/Characters/B_AlphaCharacterBase` (`self.K2_GetPawn`)))
    (`CombatComponent.SetAming` (`AlphaCharacter.Combat` _asb_alpha_character_base) true))
  (:`Completed`
    (bind _asb_alpha_character_base_2 (cast `/Game/Blueprints/Characters/B_AlphaCharacterBase` (`self.K2_GetPawn`)))
    (`CombatComponent.SetAming` (`AlphaCharacter.Combat` _asb_alpha_character_base_2) false)))

(event `EnhancedInput|/Game/Input/IA_Fire`
  (params (ActionValue :type Boolean) (ElapsedSeconds :type "Float (double-precision)") (TriggeredSeconds :type "Float (double-precision)") (InputAction :type "InputAction Object Reference" :default "/Game/Input/IA_Fire.IA_Fire"))
  (:`Started`
    (bind _asb_alpha_character_base (cast `/Game/Blueprints/Characters/B_AlphaCharacterBase` (`self.K2_GetPawn`)))
    (`CombatComponent.FireButtonPressed` (`AlphaCharacter.Combat` _asb_alpha_character_base) true))
  (:`Canceled`
    (bind _asb_alpha_character_base_2 (cast `/Game/Blueprints/Characters/B_AlphaCharacterBase` (`self.K2_GetPawn`) :!label _label))
    (`CombatComponent.FireButtonPressed` (`AlphaCharacter.Combat` _asb_alpha_character_base_2) false))
  (:`Completed`
    (goto _label)))

(fn `UserConstructionScript`)